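; BP_GunEnemy is an enemy actor with an HP bar shown through a widget component.
; On BeginPlay it casts the widget to UI_EnemyHPBar and sets full health.
; Capsule overlaps with actors tagged PlayerProjectile subtract a fixed amount from the bar's current HP.
; Health is stored only in the widget, and the Blueprint has no death handling.
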(event `self.ReceiveBeginPlay`
  (bind _asui_enemy_hpbar (cast `/Game/MyFPS/UI/UI_EnemyHPBar` (`WidgetComponent.GetWidget` (`self.WidgetComponent`))))
  (bind _output_get (set `/Game/MyFPS/UI/UI_EnemyHPBar.MaxHp` 100.0 _asui_enemy_hpbar))
  (set `/Game/MyFPS/UI/UI_EnemyHPBar.CurHp` _output_get _asui_enemy_hpbar))

(event `self.ReceiveActorBeginOverlap`
  (params (OtherActor :type "Actor Object Reference")))

(event `self.CapsuleComponent.OnComponentBeginOverlap`
  (params (OverlappedComponent :type "PrimitiveComponent Object Reference") (OtherActor :type "Actor Object Reference") (OtherComp :type "PrimitiveComponent Object Reference") (OtherBodyIndex :type Integer) (bFromSweep :type Boolean) (SweepResult :type "HitResult Structure (by ref)"))
  (if (`KismetArrayLibrary.Array_Contains` (`Actor.Tags` OtherActor) "PlayerProjectile")
    (bind _asui_enemy_hpbar (cast `/Game/MyFPS/UI/UI_EnemyHPBar` (`WidgetComponent.GetWidget` (`self.WidgetComponent`))))
    (set `/Game/MyFPS/UI/UI_EnemyHPBar.CurHp` (- (`/Game/MyFPS/UI/UI_EnemyHPBar.CurHp` _asui_enemy_hpbar) 10.0) _asui_enemy_hpbar)))

(fn `UserConstructionScript`)