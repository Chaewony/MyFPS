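; AI controller for the gun enemy that starts the BT_GunEnemy behavior tree on BeginPlay.
; On perception updates it identifies the stimulus's sense by class display name and writes the actor to the ViewingTargetActor or HearingTargetActor blackboard key.
; Any other sense clears both keys, and the handler does not check whether the stimulus was successfully sensed or lost.
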(event `self.ReceiveBeginPlay`
  (`self.RunBehaviorTree` "/Game/MyFPS/Enemy/BT_GunEnemy.BT_GunEnemy"))

(event `self.AIPerception.OnTargetPerceptionUpdated`
  (params (Actor :type "Actor Object Reference") (Stimulus :type "AIStimulus Structure"))
  (bind _returnvalue (`AIPerceptionSystem.GetSenseClassForStimulus` Stimulus))
  (switch `string` (`KismetSystemLibrary.GetClassDisplayName` _returnvalue)
    (:`Default`
      (`BlackboardComponent.SetValueAsObject` (`self.Blackboard`) "HearingTargetActor" null)
      (`BlackboardComponent.SetValueAsObject` (`self.Blackboard`) "ViewingTargetActor" null))
    (:`AISense_Sight`
      (`BlackboardComponent.SetValueAsObject` (`self.Blackboard`) "ViewingTargetActor" Actor))
    (:`AISense_Hearing`
      (`BlackboardComponent.SetValueAsObject` (`self.Blackboard`) "HearingTargetActor" Actor))))

(fn `UserConstructionScript`)